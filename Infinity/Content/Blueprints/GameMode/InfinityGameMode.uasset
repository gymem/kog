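; InfinityGameMode is a game mode that gives the player endless respawns.
; On BeginPlay it binds a respawn event to the destruction of the first player's pawn.
; When that pawn is destroyed, it spawns a new PlayerCharacter at a player start, has the first player controller possess it, and rebinds the destroyed event so the cycle repeats.
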(event Custom|RespawnPlayerCharacter
  (params (DestroyedActor :type Actor%20Object%20Reference))
  (bind _returnvalue (Game|SpawnActorfromClass "/Game/Blueprints/Player/PlayerCharacter.PlayerCharacter_C" (Transformation|GetActorTransform (Class|GameModeBase|FindPlayerStart)) "Undefined" 0 0))
  (if (Utilities|IsValid _returnvalue)
    (Pawn|Possess (Game|GetPlayerController 0) _returnvalue)
    (Game|BindEventtoOnDestroyed _returnvalue (delegate Custom|RespawnPlayerCharacter))))

(event EventBeginPlay
  (Game|BindEventtoOnDestroyed (Game|Player|GetPlayerPawn 0) (delegate Custom|RespawnPlayerCharacter)))

(event EventTick
  (params (DeltaSeconds :type Float%20%28single-precision%29)))

(fn ConstructionScript)