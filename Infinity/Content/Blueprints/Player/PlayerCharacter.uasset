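; PlayerCharacter is the player-controlled character, with camera-relative movement, look input and a placeholder gun and game-over flow.
; Axis inputs move it along the Camera's forward and right vectors and feed controller pitch and yaw.
; BeginPlay temporarily force-equips a spawned BaseGun by attaching it to the Mesh, pending item acquisition and socket-based placement.
; Any damage immediately prints "Game Over" and destroys the character.
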(event EventBeginPlay
  ;[1 1 1] 装備を入手する処理がまだないのでゲーム開始時に強制装備（仮処理）。装備位置も仮。素材のソケットから装備位置を判定できるようにする
  (bind _returnvalue (Game|SpawnActorfromClass "/Game/Blueprints/Equip/Gun/BaseGun.BaseGun_C" (Transformation|GetActorTransform) "Undefined" 0 0))
  (Transformation|AttachComponentToComponent _returnvalue (Variables|Character|GetMesh) "None" "KeepWorld" "KeepRelative" "KeepRelative" true))

(event Collision|EventActorBeginOverlap
  (params (OtherActor :type Actor%20Object%20Reference)))

(event EventTick
  (params (DeltaSeconds :type Float%20%28single-precision%29))
  ;[1 1 1] 装備を入手する処理がまだないのでゲーム開始時に強制装備（仮処理）。装備位置も仮。素材のソケットから装備位置を判定できるようにする
)

(event Game|Damage|EventAnyDamage
  (params (Damage :type Float%20%28single-precision%29) (DamageType :type Damage%20Type%20Object%20Reference) (InstigatedBy :type Controller%20Object%20Reference) (DamageCauser :type Actor%20Object%20Reference))
  (Development|PrintString "Game Over") ; 仮ゲームオーバー表示
  (Actor|DestroyActor))

(event Input|AxisEvents|InputAxisMoveForward
  (params (AxisValue :type Float%20%28single-precision%29))
  (Pawn|Input|AddMovementInput (Math|Vector|GetForwardVector (Variables|Default|GetCamera)) AxisValue false))

(event Input|AxisEvents|InputAxisMoveRight
  (params (AxisValue :type Float%20%28single-precision%29))
  (Pawn|Input|AddMovementInput (Math|Vector|GetRightVector (Variables|Default|GetCamera)) AxisValue false))

(event Input|AxisEvents|InputAxisLookUp
  (params (AxisValue :type Float%20%28single-precision%29))
  (Pawn|Input|AddControllerPitchInput AxisValue))

(event Input|AxisEvents|InputAxisTurn
  (params (AxisValue :type Float%20%28single-precision%29))
  (Pawn|Input|AddControllerYawInput AxisValue))

(fn ConstructionScript)